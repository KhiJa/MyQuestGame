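; BP_MoveableBox is an interactable box actor that attaches itself to the interacting player.
; Interact enables physics on the Cube, switches player controller 0 to Game and UI input, snaps the actor's location to the Player and sets IsActivated.
; While activated, Tick only prints the scene root's world offset from the player as debug output.
; No release or detach logic is present.
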(event `/Game/FirstPersonBP/i_Interact.Interact`
  (params (Player :type "Character Object Reference"))
  (`PrimitiveComponent.SetSimulatePhysics` (`self.Cube`) true)
  (`WidgetBlueprintLibrary.SetInputMode_GameAndUIEx` (`GameplayStatics.GetPlayerController` 0) null)
  (`self.K2_AttachToActor` Player "None" "SnapToTarget" "KeepRelative" "KeepRelative")
  (set `self.isActivated` true))

(event `self.ReceiveTick`
  (params (DeltaSeconds :type "Float (single-precision)"))
  (if (`self.isActivated`)
    (bind _output_get (set `self.offset` (- (`SceneComponent.K2_GetComponentLocation` (`self.DefaultSceneRoot`)) (`SceneComponent.K2_GetComponentLocation` (`Actor.RootComponent` (stale `/Game/FirstPersonBP/i_Interact.Interact` Player))))))
    (`KismetSystemLibrary.PrintString` (`KismetStringLibrary.Conv_VectorToString` _output_get))))

(fn `UserConstructionScript`)