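; Grabbable physics prop that the player picks up and drops with Interact, toggling between grab and release.
; Grabbing attaches the static mesh to a Physics Handle using the player camera's rotation and blocks the character's jump.
; Tick keeps the handle target a fixed distance in front of the camera.
; Releasing re-enables jumping and moves the scene root to the mesh's location.
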(event `Release`
  (`PhysicsHandleComponent.ReleaseComponent` (`self.PhysicsHandle`))
  (set `self.isGrabbed` false)
  (`SceneComponent.K2_SetWorldLocation` (`self.DefaultSceneRoot`) (`SceneComponent.K2_GetComponentLocation` (`self.StaticMesh`)) false false)
  (`/Game/DoorLever/FirstPersonCharacter.UnblockJump` (stale `/Game/I_Interact.Interact` Character)))

(event `Grab`
  (bind _staticmesh (`self.StaticMesh`))
  (`PhysicsHandleComponent.GrabComponentAtLocationWithRotation` (`self.PhysicsHandle`) _staticmesh "None" (`SceneComponent.K2_GetComponentLocation` _staticmesh) (`SceneComponent.K2_GetComponentRotation` (`self.GetComponentByClass` (`GameplayStatics.GetPlayerPawn` 0) "/Script/Engine.CameraComponent")))
  (set `self.isGrabbed` true)
  (`/Game/DoorLever/FirstPersonCharacter.BlockJump` (stale `/Game/I_Interact.Interact` Character)))

(event `/Game/I_Interact.Interact`
  (params (Character :type "/Game/DoorLever/FirstPersonCharacter Object Reference"))
  (if (`self.isGrabbed`)
    (`self.Release`)
    (else
      (`self.Grab`))))

(event `self.ReceiveTick`
  (params (DeltaSeconds :type "Float (single-precision)"))
  (bind _returnvalue (`self.GetComponentByClass` (`GameplayStatics.GetPlayerPawn` 0) "/Script/Engine.CameraComponent"))
  (`PhysicsHandleComponent.SetTargetLocation` (`self.PhysicsHandle`) (+ (`SceneComponent.K2_GetComponentLocation` _returnvalue) (* (`KismetMathLibrary.GetForwardVector` (`SceneComponent.K2_GetComponentRotation` _returnvalue)) 250.0))))

(fn `UserConstructionScript`)