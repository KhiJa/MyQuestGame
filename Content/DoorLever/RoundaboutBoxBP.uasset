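; Roundabout box actor that moves in an endless loop through a list of world-space points while activated by an OnInteract event.
; A timeline lerps the root from the stored previous position to the next point.
; When each leg finishes, it saves the position, advances the index with wraparound and restarts the timeline.
; Deactivation stops the timeline in place, so reactivation resumes the current leg.
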(event `self.ReceiveBeginPlay`
  (set `self.PrevPoint` (`SceneComponent.K2_GetComponentLocation` (`self.DefaultSceneRoot`))))

(event `/Game/DoorLever/Iinteractable.OnInteract`
  (params (isActivated :type Boolean) (id :type Integer))
  (if isActivated
    (bind (_direction _newtrack_0) (`Timeline|Timeline_0` :!label _label)
      (:`Update`
        (`SceneComponent.K2_SetWorldLocation` (`self.DefaultSceneRoot`) (`KismetMathLibrary.VLerp` (`self.PrevPoint`) (`|GetArrayItem` (`self.Points`) (`self.nextPoint`)) _newtrack_0) false false))
      (:`Finished`
        (set `self.PrevPoint` (`SceneComponent.K2_GetComponentLocation` (`self.DefaultSceneRoot`)))
        (if (== (+ (`self.nextPoint`) 1) (`KismetArrayLibrary.Array_Length` (`self.Points`)))
          (set `self.nextPoint` 0)
          (goto _label :!via `PlayFromStart`)
          (else
            (`/Engine/EditorBlueprintResources/StandardMacros.IncrementInt` (`self.nextPoint`)
              (:`  `
                (goto _label :!via `PlayFromStart`)))))))
    (else
      (goto _label :!via `Stop`))))

(fn `UserConstructionScript`)